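; BP_ComboObstacle_Master is, by its name, the base Blueprint for combo obstacles that award score when the player touches them.
; When the player character begins overlapping its Box, it passes its Type and Point variables to the game mode's SetScoreMessage.
; It then sets IsDestroyed so it scores only once; the actor itself is not destroyed here.
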(event OnComponentBeginOverlap(Box)
  (params (OverlappedComponent :type Primitive%20Component%20Object%20Reference) (OtherActor :type Actor%20Object%20Reference) (OtherComp :type Primitive%20Component%20Object%20Reference) (OtherBodyIndex :type Integer) (bFromSweep :type Boolean) (SweepResult :type Hit%20Result%20Structure%20%28by%20ref%29))
  (if (and (== OtherActor (Game|GetPlayerCharacter 0)) (not (Variables|Default|GetisDestroyed)))
    (Class|BPICombo|SetScore(Message) (Game|GetGameMode) (Variables|Default|GetType) (Variables|Default|GetPoint))
    (Variables|Default|SetisDestroyed true)))

(fn ConstructionScript)