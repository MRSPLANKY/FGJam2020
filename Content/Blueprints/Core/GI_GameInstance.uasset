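; GI_GameInstance is the game instance that holds the final score and game-over flag.
; The SetSendScore event stores the passed score and sets the game-over flag, while SetNewGame clears that flag without resetting the score.
; GetScore and GetGameOver expose those values, and GetComboTimer is a stub that always returns zero.
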(event EventSetSendScore
  (params (CurrentMultiplier :type Float%20%28single-precision%29) (CurrentScore :type Float%20%28single-precision%29) (CurrentComboScore :type Float%20%28single-precision%29))
  (Variables|Default|Setscore CurrentScore)
  (Variables|Default|SetisGameOver true))

(event EventSetNewGame
  (Variables|Default|SetisGameOver false))

(fn GetComboTimer
  (return 0.0))

(fn GetGameOver
  (return (Variables|Default|GetisGameOver)))

(fn GetScore
  (return (Variables|Default|Getscore)))